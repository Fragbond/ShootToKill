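; BP_Rifle is a rifle pickup that gives the player a rifle when collected.
; Its Pickup component's OnPickup event casts to BP_PlayerCharacter, then the rifle weapon component attaches to that character whether or not they already have a rifle.
; For a player without a rifle, it also stores that component as PlayerRifle and puts away the pistol if the player has one.
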(event `self.Pickup.OnPickup`
  (params (PickupCharacter :type "ShootToKillPlayerCharacter Object Reference"))
  (bind _asbp_player_character (cast `/Game/Blueprints/Assets/CharacterModels/Player/BP_PlayerCharacter` PickupCharacter))
  (if (`ShootToKillPlayerCharacter.HasRifle` _asbp_player_character)
    (`WeaponComponentRife.AttachRifle` (`self.WeaponComponentRife`) PickupCharacter)
    (else
      (`WeaponComponentRife.AttachRifle` (`self.WeaponComponentRife`) PickupCharacter)
      (set `/Game/Blueprints/Assets/CharacterModels/Player/BP_PlayerCharacter.PlayerRifle` (`self.WeaponComponentRife`) _asbp_player_character)
      (if (`ShootToKillPlayerCharacter.bHasPistol` _asbp_player_character)
        (`WeaponComponentPistol.PutAwayPistol` (`/Game/Blueprints/Assets/CharacterModels/Player/BP_PlayerCharacter.PlayersPistol` _asbp_player_character))))))

(fn `UserConstructionScript`)