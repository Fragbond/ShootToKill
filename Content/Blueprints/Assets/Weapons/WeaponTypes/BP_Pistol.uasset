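; BP_Pistol is a pistol weapon pickup that equips the player character on pickup.
; Its Pickup component's OnPickup event casts to BP_PlayerCharacter and always calls AttachPistol on WeaponComponentPistol.
; If the player has no pistol yet, it also stores that component as PlayersPistol and puts away any rifle the player has.
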(event `self.Pickup.OnPickup`
  (params (PickupCharacter :type "ShootToKillPlayerCharacter Object Reference"))
  (bind _weaponcomponentpistol (`self.WeaponComponentPistol`))
  (bind _asbp_player_character (cast `/Game/Blueprints/Assets/CharacterModels/Player/BP_PlayerCharacter` PickupCharacter))
  (if (`ShootToKillPlayerCharacter.bHasPistol` _asbp_player_character)
    (`WeaponComponentPistol.AttachPistol` (`self.WeaponComponentPistol`) PickupCharacter)
    (else
      (`WeaponComponentPistol.AttachPistol` _weaponcomponentpistol PickupCharacter)
      (set `/Game/Blueprints/Assets/CharacterModels/Player/BP_PlayerCharacter.PlayersPistol` _weaponcomponentpistol _asbp_player_character)
      (if (`ShootToKillPlayerCharacter.bHasRifle` _asbp_player_character)
        (`WeaponComponentRife.PutAwayRifle` (`/Game/Blueprints/Assets/CharacterModels/Player/BP_PlayerCharacter.PlayerRifle` _asbp_player_character))))))

(fn `UserConstructionScript`)