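; Sniper rifle weapon actor that the player character collects through its Pickup component.
; On pickup it casts to BP_PlayerCharacter and has WeaponComponentSniper attach the sniper, whether or not the player already has one.
; For a first sniper it also stores the component as PlayerSniper and puts away the pistol, or the rifle if the player has no pistol.
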(event `self.Pickup.OnPickup`
  (params (PickupCharacter :type "ShootToKillPlayerCharacter Object Reference"))
  (bind _asbp_player_character (cast `/Game/Blueprints/Assets/CharacterModels/Player/BP_PlayerCharacter` PickupCharacter))
  (if (`ShootToKillPlayerCharacter.HasSniper` _asbp_player_character)
    (`WeaponComponentSniper.AttachSniper` (`self.WeaponComponentSniper`) PickupCharacter)
    (else
      (`WeaponComponentSniper.AttachSniper` (`self.WeaponComponentSniper`) PickupCharacter)
      (set `/Game/Blueprints/Assets/CharacterModels/Player/BP_PlayerCharacter.PlayerSniper` (`self.WeaponComponentSniper`) _asbp_player_character)
      (if (`ShootToKillPlayerCharacter.bHasPistol` _asbp_player_character)
        (`WeaponComponentPistol.PutAwayPistol` (`/Game/Blueprints/Assets/CharacterModels/Player/BP_PlayerCharacter.PlayersPistol` _asbp_player_character))
        (elif (`ShootToKillPlayerCharacter.HasRifle` _asbp_player_character)
          (`WeaponComponentRife.PutAwayRifle` (`/Game/Blueprints/Assets/CharacterModels/Player/BP_PlayerCharacter.PlayerRifle` _asbp_player_character)))))))

(fn `UserConstructionScript`)