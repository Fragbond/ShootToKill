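; Small health pack pickup actor that players, AI, squad leaders and snipers can collect.
; It handles a separate Pickup event for each character type, calls that character's PickupSmallHealthPack, then destroys itself.
; For the three AI types it also clears the IsLowOnHealth blackboard key so their behavior stops treating them as low on health.
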(event `self.Pickup.OnPickup`
  (params (PickupCharacter :type "ShootToKillPlayerCharacter Object Reference"))
  (`ShootToKillPlayerCharacter.PickupSmallHealthPack` PickupCharacter)
  (`self.K2_DestroyActor`))

(event `self.Pickup.OnAiPickup`
  (params (AiPickupCharacter :type "ShootToKillEnemyRiflemenCharacter Object Reference"))
  (`ShootToKillEnemyRiflemenCharacter.PickupSmallHealthPack` AiPickupCharacter)
  (`BlackboardComponent.SetValueAsBool` (`AIBlueprintHelperLibrary.GetBlackboard` AiPickupCharacter) "IsLowOnHealth" false)
  (`self.K2_DestroyActor`))

(event `self.Pickup.OnSquadLeaderPickup`
  (params (SquadLeaderCharacter :type "STKSquadLeaderCharacter Object Reference"))
  (`STKSquadLeaderCharacter.PickupSmallHealthPack` SquadLeaderCharacter)
  (`BlackboardComponent.SetValueAsBool` (`AIBlueprintHelperLibrary.GetBlackboard` SquadLeaderCharacter) "IsLowOnHealth" false)
  (`self.K2_DestroyActor`))

(event `self.Pickup.OnSniperPickup`
  (params (SniperCharacter :type "STKSniper Object Reference"))
  (`STKSniper.PickupSmallHealthPack` SniperCharacter)
  (`BlackboardComponent.SetValueAsBool` (`AIBlueprintHelperLibrary.GetBlackboard` SniperCharacter) "IsLowOnHealth" false)
  (`self.K2_DestroyActor`))

(fn `UserConstructionScript`)