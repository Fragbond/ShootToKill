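; Enemy rifleman AI pawn that carries a rifle and reports what it senses and its health to a Blackboard.
; On BeginPlay the rifle weapon component attaches a weapon to the pawn.
; AI Perception updates player visibility and target, while Pawn Sensing noise events flag the player as heard.
; Tick flags low health at 20 hitpoints or below; neither that flag nor the hearing flag is cleared here.
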(event `self.ReceiveTick`
  (params (DeltaSeconds :type "Float (single-precision)"))
  (if (<= (`self.Hitpoints`) 20)
    (`BlackboardComponent.SetValueAsBool` (`AIBlueprintHelperLibrary.GetBlackboard` null) "IsLowOnHealth" true)))

(event `self.ReceiveBeginPlay`
  (`WeaponComponentRife.AttachWeaponToAi` (`self.WeaponComponentRife`) self))

(event `self.AIPerception.OnTargetPerceptionUpdated`
  (params (Actor :type "Actor Object Reference") (Stimulus :type "AIStimulus Structure"))
  (bind _returnvalue (`AIBlueprintHelperLibrary.GetBlackboard` null))
  (cast `ShootToKillPlayerCharacter` Actor)
  (`BlackboardComponent.SetValueAsBool` _returnvalue "CanSeePlayer" (`.bSuccessfullySensed` (break `AIStimulus` Stimulus)))
  (`BlackboardComponent.SetValueAsObject` _returnvalue "Target" Actor))

(event `self.PawnSensing.OnHearNoise`
  (params (Instigator :type "Pawn Object Reference") (Location :type "Vector Structure (by ref)") (Volume :type "Float (single-precision)"))
  (`BlackboardComponent.SetValueAsBool` (`AIBlueprintHelperLibrary.GetBlackboard` null) "CanHearPlayer" true))

(fn `UserConstructionScript`)