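; Sniper AI character that attaches its weapon through a sniper weapon component on spawn and feeds combat state to its Blackboard.
; Tick destroys it once dead, or flags low health when hitpoints drop to the threshold.
; Perception updates involving the player write visibility and target to the Blackboard.
; Those updates always mark the player as spotted, even when sensing is lost.
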(event `self.ReceiveBeginPlay`
  (`WeaponComponentSniper.AttachWeaponToSniper` (`self.WeaponComponentSniper`) self))

(event `self.ReceiveTick`
  (params (DeltaSeconds :type "Float (single-precision)"))
  (if (`self.IsDead`)
    (`self.K2_DestroyActor`)
    (elif (<= (`self.Hitpoints`) 25)
      (`BlackboardComponent.SetValueAsBool` (`AIBlueprintHelperLibrary.GetBlackboard` null) "IsLowOnHealth" true))))

(event `self.AIPerception.OnTargetPerceptionUpdated`
  (params (Actor :type "Actor Object Reference") (Stimulus :type "AIStimulus Structure"))
  (bind _returnvalue (`AIBlueprintHelperLibrary.GetBlackboard` null))
  (bind _asbp_player_character (cast `/Game/Blueprints/Assets/CharacterModels/Player/BP_PlayerCharacter` Actor))
  (`BlackboardComponent.SetValueAsBool` _returnvalue "CanSeePlayer" (`.bSuccessfullySensed` (break `AIStimulus` Stimulus)))
  (`BlackboardComponent.SetValueAsObject` _returnvalue "Target" Actor)
  (set `/Game/Blueprints/Assets/CharacterModels/Player/BP_PlayerCharacter.IsPlayerSpotted` true _asbp_player_character))

(fn `UserConstructionScript`)