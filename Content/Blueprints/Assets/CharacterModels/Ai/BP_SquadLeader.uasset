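; BP_SquadLeader is an AI squad leader character that detects the player and drops rifle ammo when it dies.
; On BeginPlay its rifle weapon component attaches the weapon to it.
; Perception updates on the player write CanSeePlayer and Target to the Blackboard and set the player's IsPlayerSpotted flag, which is never cleared here.
; Tick polls IsDead, then destroys the actor and spawns the ammo pickup at its transform.
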(event `self.ReceiveTick`
  (params (DeltaSeconds :type "Float (single-precision)"))
  (if (`self.IsDead`)
    (`self.K2_DestroyActor`)
    (`|SpawnActorFromClass` "/Game/Blueprints/Assets/Weapons/AmmoTypes/BP_ShootToKillRifeAmmo.BP_ShootToKillRifeAmmo_C" (`self.GetTransform`) "Undefined" "OverrideRootScale" null null)))

(event `self.ReceiveBeginPlay`
  (`WeaponComponentRife.AttachWeaponToSquadLeader` (`self.WeaponComponentRife`) self))

(event `self.AIPerception.OnTargetPerceptionUpdated`
  (params (Actor :type "Actor Object Reference") (Stimulus :type "AIStimulus Structure"))
  (bind _returnvalue (`AIBlueprintHelperLibrary.GetBlackboard` null))
  (bind _asbp_player_character (cast `/Game/Blueprints/Assets/CharacterModels/Player/BP_PlayerCharacter` Actor))
  (`BlackboardComponent.SetValueAsBool` _returnvalue "CanSeePlayer" (`.bSuccessfullySensed` (break `AIStimulus` Stimulus)))
  (`BlackboardComponent.SetValueAsObject` _returnvalue "Target" Actor)
  (set `/Game/Blueprints/Assets/CharacterModels/Player/BP_PlayerCharacter.IsPlayerSpotted` true _asbp_player_character)
  (`KismetSystemLibrary.PrintString` "Hello"))

(fn `UserConstructionScript`)